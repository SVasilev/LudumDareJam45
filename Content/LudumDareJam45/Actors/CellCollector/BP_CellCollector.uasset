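; BP_CellCollector is a goal actor that scores cells entering its box and advances the level.
; Each BP_Cell overlap increments the TopDownCharacter's Score and plays a sound.
; A looping timer opens the mapped next level when Score equals WBP_Level's required score and no BP_Cell actors remain.
; Despite its name, CheckAllCellsVelocityNearZero only tests for zero cells, as its velocity loop is unconnected.
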(event OnComponentBeginOverlap(Box)
  (params (OverlappedComponent :type Primitive%20Component%20Object%20Reference) (OtherActor :type Actor%20Object%20Reference) (OtherComp :type Primitive%20Component%20Object%20Reference) (OtherBodyIndex :type Integer) (bFromSweep :type Boolean) (SweepResult :type Hit%20Result%20Structure%20%28by%20ref%29))
  (Utilities|Casting|CastToBP_Cell OtherActor)
  (bind _astop_down_character (Utilities|Casting|CastToTopDownCharacter (Game|Player|GetPlayerPawn 0)))
  (Math|Integer|IncrementInt (Variables|/Game/LudumDareJam45/TopDownController/TopDownCharacter.TopDownCharacter_C|GetScore _astop_down_character)
    (:%20%20
      (Audio|PlaySound2D "/Game/LudumDareJam45/Audio/in_flask.in_flask" 1e+01))))

(event EventBeginPlay
  (Utilities|Time|SetTimerbyFunctionName 0 "CheckForLevelEnding" 1.0 true))

(fn ConstructionScript)

(fn CheckforLevelEnding
  (bind _astop_down_character (Utilities|Casting|CastToTopDownCharacter (Game|Player|GetPlayerPawn 0)))
  (bind _foundwidgets (Widget|GetAllWidgetsOfClass "/Game/LudumDareJam45/UI/Level/Blueprints/WBP_Level.WBP_Level_C" true))
  (bind _returnvalue (Game|GetCurrentLevelName true))
  (bind _yes (CallFunction|CheckAllCellsVelocityNearZero))
  (if (and _yes (== (Variables|/Game/LudumDareJam45/TopDownController/TopDownCharacter.TopDownCharacter_C|GetScore _astop_down_character) (.Value (Utilities|Map|Find (Variables|/Game/LudumDareJam45/UI/Level/Blueprints/WBP_Level.WBP_Level_C|GetLevelRequiredScore (Utilities|Array|Get(acopy) _foundwidgets)) _returnvalue))))
    (bind _returnvalue_2 (Game|GetCurrentLevelName true))
    (Game|OpenLevel(byName) (.Value (Utilities|Map|Find (Variables|Default|GetNextLevel) _returnvalue_2)))))

(fn CheckAllCellsVelocityNearZero
  (bind _outactors (Actor|GetAllActorsOfClass "/Game/LudumDareJam45/Actors/Cell/Blueprints/BP_Cell.BP_Cell_C"))
  (if (== (Utilities|Array|Length _outactors) 0)
    (return true)
    (else
      (return false))))