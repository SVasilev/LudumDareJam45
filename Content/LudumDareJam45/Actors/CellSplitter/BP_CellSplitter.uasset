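; BP_CellSplitter is an actor that splits any BP_Cell touching its sphere collision into two smaller cells.
; On overlap it destroys the incoming cell and calls SplitCell once per side along Y.
; SplitCell spawns a half-scale BP_Cell offset sideways, enables physics locked to the YZ plane, and launches it outward and slightly downward.
; An unconnected copy of the spawn logic remains in the EventGraph and never runs.
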(event OnComponentBeginOverlap(SphereCollision)
  (params (OverlappedComponent :type Primitive%20Component%20Object%20Reference) (OtherActor :type Actor%20Object%20Reference) (OtherComp :type Primitive%20Component%20Object%20Reference) (OtherBodyIndex :type Integer) (bFromSweep :type Boolean) (SweepResult :type Hit%20Result%20Structure%20%28by%20ref%29))
  (bind _asbp_cell (Utilities|Casting|CastToBP_Cell OtherActor))
  (Actor|DestroyActor _asbp_cell)
  (CallFunction|SplitCell 1.0)
  (CallFunction|SplitCell -1.0))

(fn ConstructionScript)

(fn SplitCell
  (params (Direction :type Float%20%28single-precision%29))
  (bind _spherecollision (Variables|Default|GetSphereCollision))
  (bind _returnvalue (Transformation|GetWorldLocation _spherecollision))
  (bind _returnvalue_2 (Game|SpawnActorfromClass "/Game/LudumDareJam45/Actors/Cell/Blueprints/BP_Cell.BP_Cell_C" (Math|Transform|MakeTransform (Math|Vector|MakeVector (.x _returnvalue) (+ (* Direction 3e+01) (.y _returnvalue)) (.z _returnvalue)) "0, 0, 0" "0.500000,0.500000,0.500000") "Undefined" 0 0))
  (Physics|SetSimulatePhysics (Variables|/Game/LudumDareJam45/Actors/Cell/Blueprints/BP_Cell.BP_Cell_C|GetSphereCollision _returnvalue_2) true)
  (Class|PrimitiveComponent|SetConstraintMode (Variables|/Game/LudumDareJam45/Actors/Cell/Blueprints/BP_Cell.BP_Cell_C|GetSphereCollision _returnvalue_2) "YZPlane")
  (Physics|SetPhysicsLinearVelocity (Variables|/Game/LudumDareJam45/Actors/Cell/Blueprints/BP_Cell.BP_Cell_C|GetSphereCollision _returnvalue_2) (Math|Vector|MakeVector 0.0 (* Direction 1.2e+02) -3e+01) false "None"))